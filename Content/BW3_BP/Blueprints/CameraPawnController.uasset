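; Player controller for an RTS-style building game, driving the camera pawn and building placement.
; On BeginPlay it spawns a construction manager and building and element ghosts, then creates the main HUD.
; Input moves, pans, zooms and edge-scrolls the camera, scaling move speed with zoom and following ground height on forward movement.
; In build mode the ghost follows the cursor, rotates, and queues non-overlapping placements; elemental mode and a V-key NPC spawn are debug stubs.
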(event `self.ReceiveTick`
  (params (DeltaSeconds :type "Float (single-precision)"))
  ;[1 1 1] Build Mode Follow Cursor
  (if (`self.BuildModeActive`)
    (`self.SetGhostBuildingToMouse`)
    (elif (`self.ElementalModeActive`)
      _)))

(event `self.ReceiveBeginPlay`
  (bind _returnvalue (`KismetMathLibrary.MakeTransform` (0.0 0.0 0.0)))
  ;[1 1 1] EventBeginPlay
  (`|ExecutionSequence`
    (:`then_0`
      (`self.ReferenceCasts`))
    (:`then_1`
      (bind _returnvalue_2 (`|SpawnActorFromClass` "/Game/BW3_BP/Blueprints/Construction/ConstructionManager_BP.ConstructionManager_BP_C" _returnvalue "AlwaysSpawn" "OverrideRootScale" null null))
      (set `self.ConstructionManagerRef` _returnvalue_2))
    (:`then_2`
      (bind _returnvalue_3 (`|SpawnActorFromClass` "/Game/BW3_BP/Blueprints/Buildings/GhostBuilding_BP.GhostBuilding_BP_C" _returnvalue "AlwaysSpawn" "OverrideRootScale" null self "/Game/Materials/GhostError_M_Inst.GhostError_M_Inst" "/Game/Materials/Ghost_M_Inst.Ghost_M_Inst" null))
      (set `self.GhostBuildingRef` _returnvalue_3))
    (:`then_3`
      (bind _returnvalue_4 (`|SpawnActorFromClass` "/Game/BW3_BP/Blueprints/Elements/GhostElement_BP.GhostElement_BP_C" _returnvalue "AlwaysSpawn" "OverrideRootScale" null self null))
      (set `self.GhostElementRef` _returnvalue_4))
    (:`then_4`
      (`WidgetBlueprintLibrary.SetInputMode_GameAndUIEx` self null "LockAlways")
      (`self.CreateHUD`)
      (set `PlayerController.bShowMouseCursor` true (`GameplayStatics.GetPlayerController` 0)))))

(event `InputAxis|MoveForward`
  (params (AxisValue :type "Float (single-precision)"))
  ;[0.7507 0.5412 1] Camera Movement
  ;;[1 1 1] Movement X
  (if (not (`self.DisableCamNav`))
    (`self.K2_SetActorTransform` (`self.CameraPawnRef`) (`KismetMathLibrary.MakeTransform` (`KismetMathLibrary.MakeVector` (.x (.location (`self.MovementX` AxisValue (`self.MovementSpeedCalculation`) (`self.FastMoveMultiplier`) (`self.CameraPawnRef`)))) (.y (.location (`self.MovementX` AxisValue (`self.MovementSpeedCalculation`) (`self.FastMoveMultiplier`) (`self.CameraPawnRef`)))) (`self.RecalculateZ`)) (.rotation (`self.MovementX` AxisValue (`self.MovementSpeedCalculation`) (`self.FastMoveMultiplier`) (`self.CameraPawnRef`))) (.scale (`self.MovementX` AxisValue (`self.MovementSpeedCalculation`) (`self.FastMoveMultiplier`) (`self.CameraPawnRef`)))) false false)))

(event `InputAxisKey|MouseX`
  (params (AxisValue :type "Float (single-precision)"))
  ;[0.7507 0.5412 1] Camera Movement
  ;;[1 1 1] Camera Yaw
  (`/Engine/EditorBlueprintResources/StandardMacros.Gate` true :!label _label
    (:`Exit`
      (`self.K2_SetActorRotation` (`self.CameraPawnRef`) (`KismetMathLibrary.MakeRotator` (.roll (`self.K2_GetActorRotation` (`self.CameraPawnRef`))) (.pitch (`self.K2_GetActorRotation` (`self.CameraPawnRef`))) (+ (.yaw (`self.K2_GetActorRotation` (`self.CameraPawnRef`))) (* AxisValue (`self.PanSensitivity`)))) false))))

(event `InputAction|Pan`
  (params (Key :type "Key Structure"))
  ;[0.7507 0.5412 1] Camera Movement
  ;;[1 1 1] Camera Yaw
  (:`Pressed`
    (set `self.DisableCamNav` true)
    (goto _label :!via `Open`))
  (:`Released`
    (set `self.DisableCamNav` false)
    (goto _label :!via `Close`)))

(event `InputAxis|MoveRight`
  (params (AxisValue :type "Float (single-precision)"))
  ;[0.7507 0.5412 1] Camera Movement
  ;;[1 1 1] Movement Y
  (if (not (`self.DisableCamNav`))
    (`self.K2_SetActorTransform` (`self.CameraPawnRef`) (`self.MovementY` AxisValue (`self.MovementSpeedCalculation`) (`self.FastMoveMultiplier`) (`self.CameraPawnRef`)) false false)))

(event `Key|LeftShift`
  (params (Key :type "Key Structure"))
  ;[0.7507 0.5412 1] Camera Movement
  ;;[1 1 1] Move Multiplier
  (:`Pressed`
    (set `self.FastMoveMultiplier` 2.0))
  (:`Released`
    (set `self.FastMoveMultiplier` 1.0)))

(event `InputAction|Deselect`
  (params (Key :type "Key Structure"))
  ;[1 1 1] Deselect
  (:`Pressed`
    (if (or (`self.BuildModeActive`) (`self.ElementalModeActive`))
      (`/Game/BW3_BP/Blueprints/Buildings/GhostBuilding_BP.KillGhost` (`self.GhostBuildingRef`))
      (`/Game/BW3_BP/Blueprints/Elements/GhostElement_BP.KillGhost` (`self.GhostElementRef`)))))

(event `InputAxisKey|MouseY`
  (params (AxisValue :type "Float (single-precision)"))
  ;[0.7507 0.5412 1] Camera Movement
  ;;[1 1 1] Camera Pitch
  (`/Engine/EditorBlueprintResources/StandardMacros.Gate` true :!label _label_2
    (:`Exit`
      (`self.K2_SetActorRotation` (`self.CameraPawnRef`) (`KismetMathLibrary.MakeRotator` (.roll (`self.K2_GetActorRotation` (`self.CameraPawnRef`))) (`KismetMathLibrary.FClamp` (+ (.pitch (`self.K2_GetActorRotation` (`self.CameraPawnRef`))) (* AxisValue (`self.PanSensitivity`))) -15.0 65.0) (.yaw (`self.K2_GetActorRotation` (`self.CameraPawnRef`)))) false))))

(event `InputAction|PanReset`
  (params (Key :type "Key Structure"))
  (bind _camerapawnref (`self.CameraPawnRef`))
  ;[0.7507 0.5412 1] Camera Movement
  ;;[1 1 1] Pitch Reset
  (:`Pressed`
    (`self.K2_SetActorRotation` _camerapawnref (`KismetMathLibrary.MakeRotator` (.roll (`self.K2_GetActorRotation` _camerapawnref)) 0.0 (.yaw (`self.K2_GetActorRotation` _camerapawnref))) false)))

(event `InputAction|Pan`
  (params (Key :type "Key Structure"))
  ;[0.7507 0.5412 1] Camera Movement
  ;;[1 1 1] Camera Pitch
  (:`Pressed`
    (set `self.DisableCamNav` true)
    (goto _label_2 :!via `Open`))
  (:`Released`
    (set `self.DisableCamNav` false)
    (goto _label_2 :!via `Close`)))

(event `InputAction|Select`
  (params (Key :type "Key Structure"))
  ;[1 1 1] Select
  (:`Pressed`
    (if (`self.BuildModeActive`)
      (if (not (`/Game/BW3_BP/Blueprints/Buildings/GhostBuilding_BP.GetIsOverlapping` (`self.GhostBuildingRef`)))
        (bind _constructionstruct (`/Game/BW3_BP/Blueprints/Buildings/GhostBuilding_BP.GetConstructionStruct` (`self.GhostBuildingRef`)))
        (`/Game/BW3_BP/Blueprints/Construction/ConstructionManager_BP.QueueConstruction` (`self.ConstructionManagerRef`) _constructionstruct)
        (`/Game/BW3_BP/Blueprints/Buildings/GhostBuilding_BP.KillGhost` (`self.GhostBuildingRef`)))
      (elif (`self.ElementalModeActive`)
        (`KismetSystemLibrary.PrintString` "Fire!!")))))

(event `InputAction|ZoomReset`
  (params (Key :type "Key Structure"))
  ;[0.7507 0.5412 1] Camera Movement
  ;;[1 1 1] Zoom Reset
  (:`Pressed`
    (set `SpringArmComponent.TargetArmLength` (`self.DefaultZoom`) (`/Game/BW3_BP/Blueprints/CameraPawn.SpringArm` (`self.CameraPawnRef`)))))

(event `InputAction|ZoomIn`
  (params (Key :type "Key Structure"))
  (bind _springarm (`/Game/BW3_BP/Blueprints/CameraPawn.SpringArm` (`self.CameraPawnRef`)))
  ;[0.7507 0.5412 1] Camera Movement
  ;;[1 1 1] Camera Zoom
  (:`Pressed`
    (set `SpringArmComponent.TargetArmLength` (`KismetMathLibrary.FClamp` (- (`SpringArmComponent.TargetArmLength` _springarm) (`self.ZoomSensitivity`)) 250.0 (`self.MaxArmDistance`)) _springarm)))

(event `InputAxisKey|MouseX`
  (params (AxisValue :type "Float (single-precision)"))
  ;[0.7507 0.5412 1] Camera Movement
  ;;[1 1 1] EdgeMovement
  (if (not (`self.DisableCamNav`))
    (bind (_deltaxspeed _deltayspeed) (`self.ScreenEdgeMovement` :!label _label_3))
    (`self.K2_AddActorLocalOffset` (`self.CameraPawnRef`) (`KismetMathLibrary.MakeVector` _deltaxspeed _deltayspeed) true false)))

(event `InputAxisKey|MouseY`
  (params (AxisValue :type "Float (single-precision)"))
  ;[0.7507 0.5412 1] Camera Movement
  ;;[1 1 1] EdgeMovement
  (if (not (`self.DisableCamNav`))
    (goto _label_3 :!via `MouseY`)))

(event `InputAction|ZoomOut`
  (params (Key :type "Key Structure"))
  (bind _springarm (`/Game/BW3_BP/Blueprints/CameraPawn.SpringArm` (`self.CameraPawnRef`)))
  ;[0.7507 0.5412 1] Camera Movement
  ;;[1 1 1] Camera Zoom
  (:`Pressed`
    (set `SpringArmComponent.TargetArmLength` (`KismetMathLibrary.FClamp` (+ (`SpringArmComponent.TargetArmLength` _springarm) (`self.ZoomSensitivity`)) 250.0 (`self.MaxArmDistance`)) _springarm)))

(event `InputAction|RotateBuildingRight`
  (params (Key :type "Key Structure"))
  (bind _ghostbuildingref (`self.GhostBuildingRef`))
  (bind (_returnvalue_roll _returnvalue_pitch _returnvalue_yaw) (`KismetMathLibrary.BreakRotator` (`self.K2_GetActorRotation` _ghostbuildingref)))
  ;[1 1 1] Rotate Buildings
  (:`Pressed`
    (if (and (`KismetSystemLibrary.IsValid` _ghostbuildingref) (`self.BuildModeActive`))
      (`self.K2_SetActorRotation` (`self.GhostBuildingRef`) (`KismetMathLibrary.MakeRotator` _returnvalue_roll _returnvalue_pitch (- _returnvalue_yaw (`self.BuildingRotationRate`))) false))))

(event `Key|V`
  (params (Key :type "Key Structure"))
  (bind (_mouselocation_x _mouselocation_y) (`KismetMathLibrary.BreakVector` (`/Game/Libraries/FunctionLibrary.SetCursorWorldPosition` self (`self.SightDistance`))))
  (bind (_returnvalue_x _returnvalue_y _returnvalue_z) (`KismetMathLibrary.BreakVector` (`self.K2_GetActorLocation` (`self.CameraPawnRef`))))
  ;[1 1 1] Spawn NPC //DEBUG
  (:`Pressed`
    (bind _outhit (`KismetSystemLibrary.LineTraceSingle` (`KismetMathLibrary.MakeVector` _mouselocation_x _mouselocation_y _returnvalue_z) (`KismetMathLibrary.MakeVector` _mouselocation_x _mouselocation_y (- _returnvalue_z (`self.SightDistance`))) "TraceTypeQuery3"))
    (if (`GameplayStatics.BreakHitResult` _outhit)
      (`|SpawnActorFromClass` "/Game/BW3_BP/Blueprints/NPC/NPC_BP.NPC_BP_C" (`KismetMathLibrary.MakeTransform` (`KismetMathLibrary.MakeVector` _mouselocation_x _mouselocation_y (+ (.z (`.Location` (`GameplayStatics.BreakHitResult` _outhit))) (* 93.0 0.25)))) "Undefined" "OverrideRootScale" null null)
      (else
        (`KismetSystemLibrary.PrintString` "Miss")))))

(event `InputAction|RotateBuildingLeft`
  (params (Key :type "Key Structure"))
  (bind _ghostbuildingref (`self.GhostBuildingRef`))
  (bind (_returnvalue_roll _returnvalue_pitch _returnvalue_yaw) (`KismetMathLibrary.BreakRotator` (`self.K2_GetActorRotation` _ghostbuildingref)))
  ;[1 1 1] Rotate Buildings
  (:`Pressed`
    (if (and (`KismetSystemLibrary.IsValid` _ghostbuildingref) (`self.BuildModeActive`))
      (`self.K2_SetActorRotation` (`self.GhostBuildingRef`) (`KismetMathLibrary.MakeRotator` _returnvalue_roll _returnvalue_pitch (+ _returnvalue_yaw (`self.BuildingRotationRate`))) false))))

(fn `MovementSpeedCalculation`
  (returns (MoveSensitivity :type "Float (double-precision)"))
  (return (`KismetMathLibrary.FClamp` (/ (`SpringArmComponent.TargetArmLength` (`/Game/BW3_BP/Blueprints/CameraPawn.SpringArm` (`self.CameraPawnRef`))) 100.0) 5.0 20.0)))

(fn `RecalculateZ`
  (returns (UpdateZLocation :type "Float (double-precision)"))
  (locals (SphereLocation :type "Vector Structure" :default (0.0 0.0 0.0)))
  (bind _returnvalue (`self.K2_GetActorLocation` (`self.CameraPawnRef`)))
  (bind _output_get (set `local.SphereLocation` _returnvalue))
  (bind _outhit (`KismetSystemLibrary.LineTraceSingle` _output_get (- _returnvalue (0.0 0.0 200.0)) "TraceTypeQuery3"))
  (return (+ (.z (`.ImpactPoint` (`GameplayStatics.BreakHitResult` _outhit))) 100.0)))

(fn `SestGhostElementToMouse`
  (if (!= (`self.GhostElementRef`) null)
    (`/Game/BW3_BP/Blueprints/Elements/GhostElement_BP.SetCursorPostion` (`self.GhostElementRef`) (`/Game/Libraries/FunctionLibrary.SetCursorWorldPosition` self (`self.SetSightDistance`)))))

(fn `SetCalendar`
  (params (Date :type "Array of Integer (by ref)"))
  (returns (Success :type Boolean))
  (return false))

(fn `SetClock`
  (params (Time :type "Array of Integer (by ref)"))
  (returns (Success :type Boolean))
  (return false))

(fn `SetGhostBuildingToMouse`
  (if (!= (`self.GhostBuildingRef`) null)
    (`/Game/BW3_BP/Blueprints/Buildings/GhostBuilding_BP.SetCursorPostion` (`self.GhostBuildingRef`) (`/Game/Libraries/FunctionLibrary.SetCursorWorldPosition` self (`self.SetSightDistance`)))))

(fn `SetSightDistance`
  (returns (SightDistance :type "Float (double-precision)"))
  (return (+ (`self.SightDistance`) (`SpringArmComponent.TargetArmLength` (`/Game/BW3_BP/Blueprints/CameraPawn.SpringArm` (`self.CameraPawnRef`))))))

(fn `UserConstructionScript`)