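; NPC Blueprint that randomizes its sex, body color and name in the Construction Script.
; RandomNPCFeatures creates a dynamic material instance on the mesh, rolls a sex and sets BodyColor to the male or female color.
; GetRandomName draws a random entry from the matching male or female name enum as a string, which is stored with the sex in MyProfile.
; The event graph holds no logic.
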(fn `GetRandomName`
  (params (Sex :type "/Game/BW3_BP/Blueprints/NPC/NPC_SexType_ENUM Enum" :default "NewEnumerator0"))
  (returns (Name :type String))
  (if (`|EnumEquality` Sex "NewEnumerator0")
    (return (`|GetEnumeratorNameAsString` (enumliteral `/Game/BW3_BP/Blueprints/NPC/NPC_Name_Male_ENUM` (cast `/Game/BW3_BP/Blueprints/NPC/NPC_Name_Male_ENUM` (`KismetMathLibrary.Conv_IntToByte` (`KismetMathLibrary.RandomIntegerInRange` (- (enumcount `/Game/BW3_BP/Blueprints/NPC/NPC_Name_Male_ENUM`) 1)))))))
    (else
      (return (`|GetEnumeratorNameAsString` (enumliteral `/Game/BW3_BP/Blueprints/NPC/NPC_Name_Female_ENUM` (cast `/Game/BW3_BP/Blueprints/NPC/NPC_Name_Female_ENUM` (`KismetMathLibrary.Conv_IntToByte` (`KismetMathLibrary.RandomIntegerInRange` (- (enumcount `/Game/BW3_BP/Blueprints/NPC/NPC_Name_Female_ENUM`) 1))))))))))

(fn `RandomNPCFeatures`
  (locals (MaterialInstance :type "MaterialInstanceDynamic Object Reference") (NewLocalVar_0 :type "/Game/BW3_BP/Blueprints/NPC/NPC_SexType_ENUM Enum") (FemaleColor :type "LinearColor Structure" :default (struct :`R` 0.875 :`G` 0.123047 :`B` 0.364056)) (MaleColor :type "LinearColor Structure" :default (struct :`R` 0.005208 :`G` 0.148786 :`B` 1.0)))
  (bind _materialinstance (`local.MaterialInstance`))
  (bind _returnvalue (`PrimitiveComponent.CreateDynamicMaterialInstance` (`self.Mesh`) 0 "/Game/Materials/M_UE4Man_Body_Inst.M_UE4Man_Body_Inst"))
  (set `local.MaterialInstance` _returnvalue)
  (if (`|EnumEquality` (enumliteral `/Game/BW3_BP/Blueprints/NPC/NPC_SexType_ENUM` (cast `/Game/BW3_BP/Blueprints/NPC/NPC_SexType_ENUM` (`KismetMathLibrary.Conv_IntToByte` (`KismetMathLibrary.RandomIntegerInRange` 0 1)))) "NewEnumerator0")
    (`MaterialInstanceDynamic.SetVectorParameterValue` _materialinstance "BodyColor" (`local.MaleColor`))
    (bind _name (`self.GetRandomName` "NewEnumerator0"))
    (set `self.MyProfile` (make `/Game/BW3_BP/Blueprints/Structs/NPC_Profile_STRUCT` _name))
    (else
      (`MaterialInstanceDynamic.SetVectorParameterValue` _materialinstance "BodyColor" (`local.FemaleColor`))
      (bind _name_2 (`self.GetRandomName` "NewEnumerator1"))
      (set `self.MyProfile` (make `/Game/BW3_BP/Blueprints/Structs/NPC_Profile_STRUCT` _name_2 "NewEnumerator1")))))

(fn `UserConstructionScript`
  (`self.RandomNPCFeatures`))