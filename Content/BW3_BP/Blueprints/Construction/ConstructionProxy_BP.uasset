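; Construction proxy actor that stands in for a building under construction, showing its display mesh with a ghost material and configuring entrance and collision from that mesh.
; Each tick it accumulates work time scaled by the DayNightCycle time unit, binding to that actor's game speed dispatcher.
; Once work time reaches the construction time, it fires ConstructionCompleted with itself, then destroys itself after a short delay.
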(event `self.ReceiveBeginPlay`
  (bind _outactors (`GameplayStatics.GetAllActorsOfClass` "/Game/BW3_BP/Blueprints/DateTime_BP/DayNightCycle.DayNightCycle_C"))
  (if (> (`KismetArrayLibrary.Array_Length` _outactors) 0)
    (bind _output_get (set `self.DayNightCycle` (`|GetArrayItem` _outactors)))
    (add `/Game/BW3_BP/Blueprints/DateTime_BP/DayNightCycle.UpdateGameSpeedDispatch` _output_get (`|CreateDelegate` :!event `AdjustTime`))
    (set `self.TimeUnit` (`/Game/BW3_BP/Blueprints/DateTime_BP/DayNightCycle.TimeUnit` _output_get))))

(event `self.ReceiveTick`
  (params (DeltaSeconds :type "Float (single-precision)"))
  (bind _worktimespent (`self.WorkTimeSpent`))
  (set `self.Delta` DeltaSeconds)
  (if (not (`self.isConstructionCompleted`))
    (`self.DoWork`)
    (`KismetSystemLibrary.PrintString` (`KismetStringLibrary.Conv_DoubleToString` _worktimespent) false false)
    (if (>= _worktimespent (`self.ConstructionTime`))
      (set `self.isConstructionCompleted` true)
      (`self.ConstructionCompleted` self)
      (`KismetSystemLibrary.Delay` 0.2)
      (`self.K2_DestroyActor`))))

(event `AdjustTime`
  (params (TimeUnit :type "Float (double-precision)"))
  (set `self.TimeUnit` TimeUnit))

(fn `DoWork`
  (bind _output_get (set `self.ClockWork` (`/Game/Libraries/FunctionLibrary.SetClockWork` (`self.Delta`) (`self.TimeUnit`) (`self.ClockWork`))))
  (set `self.WorkTimeSpent` _output_get)
  (return))

(fn `SetConstructionTime`
  (params (WorkHours :type "Float (double-precision)"))
  (set `self.ConstructionTime` WorkHours)
  (return))

(fn `UserConstructionScript`
  (bind _staticmesh (`self.StaticMesh`))
  (`StaticMeshComponent.SetStaticMesh` _staticmesh (`self.DisplayMesh`))
  (`PrimitiveComponent.SetMaterial` _staticmesh 0 "/Game/Materials/Ghost_M_Inst.Ghost_M_Inst")
  (`/Game/Libraries/FunctionLibrary.SetBuildingEntrance` (`self.Entrance`) (`self.StaticMesh`))
  (`/Game/Libraries/FunctionLibrary.SetBuildingCollisionBox` (`self.Collision`) (`self.StaticMesh`)))