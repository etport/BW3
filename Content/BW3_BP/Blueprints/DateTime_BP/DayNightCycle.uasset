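; Day-night cycle Blueprint that runs the game clock and calendar, rotates the sun light and refreshes the sky sphere.
; Tick advances time drives scaled by game speed, then pushes time and date to the main UI widget.
; Sun pitch follows parabolic arcs from latitude and seasonal declination, with separate polar day/night and equator-flip handling.
; Moon declination and inclination update each day but drive no light here; UpdateGameSpeed rescales time and broadcasts it.
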(event `self.ReceiveBeginPlay`
  (bind (_timeinhours _sundeclinationdrive _sundrive) (`self.SetUserDefinedTime`))
  (bind _ascamera_pawn_controller (cast `/Game/BW3_BP/Blueprints/CameraPawnController` (`GameplayStatics.GetPlayerController` 0)))
  (bind _output_get (set `self.ControllerRef` _ascamera_pawn_controller))
  (set `self.HUDref` (`/Game/BW3_BP/Blueprints/CameraPawnController.MainUIWidget` _output_get))
  (set `self.MoonDayDuration` (/ (* (`self.SunDayDuration`) 30.0) 29.0))
  (set `self.Clockwork` _timeinhours)
  (set `self.SunDeclinationDrive` _sundeclinationdrive)
  (set `self.SunDrive` _sundrive)
  (`self.MakeGameDateArray`)
  (set `self.SunDeclination` (`self.CalculateSunDeclination`))
  (if (`self.CheckEquatorFlipSun`)
    (set `self.SunEquatorFlip` -1.0)
    (else
      (set `self.SunEquatorFlip` 1.0)))
  (set `self.SunPolar` (`self.CheckPolar`))
  (set `self.TimeUnit` (`self.DefaultGameSpeed`)))

(event `self.ReceiveTick`
  (params (DeltaSeconds :type "Float (single-precision)"))
  (bind (_clockworkout _daytick) (`/Game/Libraries/FunctionLibrary.SetClockWork` (`self.DeltaSeconds`) (`self.TimeUnit`) (`self.Clockwork`)))
  (bind _output_get (set `self.DeltaSeconds` DeltaSeconds))
  (bind _returnvalue (/ _output_get (`self.TimeUnit`)))
  (set `self.SunDrive` (+ _returnvalue (`self.SunDrive`)))
  (set `self.MoonDrive` (+ (`self.MoonDrive`) _returnvalue))
  (set `self.MoonDeclinationDrive` (/ _returnvalue (`self.MoonDayDuration`)))
  (set `self.SunDeclinationDrive` (+ (`self.SunDeclinationDrive`) (/ _returnvalue (`self.SunDayDuration`))))
  (if (>= (`self.SunDeclinationDrive`) (`self.SunYearDuration`))
    (set `self.SunDeclinationDrive` 0.0))
  (set `self.Clockwork` _clockworkout)
  (set `self.DayTick` _daytick)
  (`self.SunTrajectory`)
  (`self.K2_SetActorRotation` (`self.SunLight`) (`KismetMathLibrary.MakeRotator` 0.0 (`self.SunPitch`) (`self.SunYaw`)) false)
  (`/Game/BW3_BP/BP_SkySphere/BP_Sky_Sphere2.UpdateSunDirection` (`self.BP_SkySphere`))
  (`self.Clock`)
  (`self.Calendar`)
  (if (>= (`self.SunDrive`) (`self.SunDayDuration`))
    (set `self.SunDrive` 0.0)
    (if (`self.CheckEquatorFlipSun`)
      (set `self.SunEquatorFlip` -1.0)
      (else
        (set `self.SunEquatorFlip` 1.0)))
    (set `self.SunPolar` (`self.CheckPolar`))
    (set `self.MoonDeclination` (`self.CalculateMoonDeclination`))
    (set `self.MoonInclination` (`self.CalculateMoonInclination`))
    (if (`self.CheckEquatorFlipMoon`)
      (set `self.MoonEquatorFlip` -1.0)
      (else
        (set `self.MoonEquatorFlip` 1.0)))))

(event `/Game/BW3_BP/Blueprints/BW3Interface.UpdateGameSpeed`
  (params (Multiplier :type "Float (single-precision)"))
  (bind _output_get (set `self.TimeUnit` (* Multiplier (`self.DefaultGameSpeed`))))
  (`self.UpdateGameSpeedDispatch` _output_get))

(fn `Calendar`
  (bind _gamedate (`self.GameDate`))
  (bind _output_get (set `self.GameDay` (+ (`self.GameDay`) (`self.DayTick`))))
  (if (> _output_get (`KismetMathLibrary.DaysInMonth` (`|GetArrayItem` _gamedate 2) (`|GetArrayItem` _gamedate 1)))
    (set `self.GameDay` 1)
    (set `self.GameMonth` (+ (`self.GameMonth`) 1)))
  (if (> (`self.GameMonth`) 12)
    (set `self.GameMonth` 1)
    (set `self.GameYear` (+ (`self.GameYear`) 1)))
  (bind _output_get_2 (set `self.GameDate` (`|MakeArray` (`self.GameDay`) (`self.GameMonth`) (`self.GameYear`))))
  (message `/Game/BW3_BP/Blueprints/BW3Interface.SetCalendar` (`/Game/BW3_BP/Blueprints/CameraPawnController.MainUIWidget` (`self.ControllerRef`)) _output_get_2))

(fn `Clock`
  (bind (_remainder _returnvalue) (`KismetMathLibrary.FMod` (* (`self.Clockwork`) 3600.0) 60.0))
  (bind (_remainder_2 _returnvalue_2) (`KismetMathLibrary.FMod` (`KismetMathLibrary.Conv_IntToDouble` _returnvalue) 60.0))
  (set `self.Seconds` (`KismetMathLibrary.FFloor` _remainder))
  (set `self.Minutes` (`KismetMathLibrary.FFloor` _remainder_2))
  (set `self.Hours` (`KismetMathLibrary.FFloor` (`KismetMathLibrary.FMod` (`KismetMathLibrary.Conv_IntToDouble` _returnvalue_2) 24.0)))
  (bind _output_get (set `self.GameTime` (`|MakeArray` (`self.Seconds`) (`self.Minutes`) (`self.Hours`))))
  (message `/Game/BW3_BP/Blueprints/BW3Interface.SetClock` (`/Game/BW3_BP/Blueprints/CameraPawnController.MainUIWidget` (`self.ControllerRef`)) _output_get))

(fn `SetCalendar`
  (params (Date :type "Array of Integer (by ref)"))
  (returns (Success :type Boolean))
  (return false))

(fn `SetClock`
  (params (Time :type "Array of Integer (by ref)"))
  (returns (Success :type Boolean))
  (return false))

(fn `SunTrajectory`
  (bind (_midnight_to_sunrise _sunrise_to_sunset _sunset_to_midnight) (`self.DayNightCheck`))
  (bind (_midnight_to_sunrise_2 _sunrise_to_sunset_2 _sunset_to_midnight_2) (`self.DayNightCheckPolar`))
  (set `self.SunDeclination` (`self.CalculateSunDeclination`))
  (if (`self.SunPolar`)
    (if _midnight_to_sunrise_2
      (`self.SetDayNightFlipPolar` :!label _label
        (:`then`
          _)
        (:`then2`
          _)
        (:`then3`
          _))
      (set `self.SunPitch` (`self.CalculateSunPitchPolar`))
      (set `self.SunYaw` (+ (* (`self.SunEquatorFlip`) (/ (* (`self.SunDrive`) 360.0) (`self.SunDayDuration`))) (* (- 1.0 (`self.SunEquatorFlip`)) 2.0)) :!label _label_2)
      (elif _sunrise_to_sunset_2
        (goto _label :!via `Sunrise to Sunset`)
        (elif _sunset_to_midnight_2
          (goto _label :!via `Sunset to Midnight`))))
    (else
      (set `self.SunHalfDaylight` (`self.CalculateSunArcDay`))
      (set `self.SunHalfNight` (`self.CalculateSunArcNight`))
      (if _midnight_to_sunrise
        (`self.SetDayNightFlip` (`self.SunDayDuration`) :!label _label_3
          (:`then`
            _)
          (:`then2`
            _)
          (:`then3`
            _))
        (set `self.SunPitch` (`self.CalculateSunPitch`))
        (goto _label_2)
        (elif _sunrise_to_sunset
          (goto _label_3 :!via `Sunrise to Sunset`)
          (elif _sunset_to_midnight
            (goto _label_3 :!via `Sunset to Midnight`)))))))

(fn `UserConstructionScript`)