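; PlantMaster_BP is a plant Blueprint, apparently a master for plant buildings, that animates its mesh growing after it spawns.
; On BeginPlay it shrinks the static mesh to a tenth of its size, then plays the PlantGrow timeline at a play rate set by GrowRate.
; Each timeline update applies the Scale track uniformly to the mesh's world scale.
; The construction script only calls the parent's.
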(event `self.ReceiveBeginPlay`
  (`SceneComponent.SetWorldScale3D` (`self.StaticMesh`) (0.1 0.1 0.1))
  (`TimelineComponent.SetPlayRate` (`self.PlantGrow`) (`self.GrowRate`))
  (bind (_direction _scale) (`Timeline|PlantGrow`)
    (:`Update`
      (`SceneComponent.SetWorldScale3D` (`self.StaticMesh`) (`KismetMathLibrary.MakeVector` _scale _scale _scale)))))

(fn `UserConstructionScript`
  (`parent.UserConstructionScript`))